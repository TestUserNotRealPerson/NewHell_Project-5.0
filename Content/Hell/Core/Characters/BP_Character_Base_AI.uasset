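; Base AI bot character: loads settings by bot name from a data table and runs an overridable state machine on a looping timer.
; A timed distance, view-cone and trace check detects the player.
; The FoundedPlayer RepNotify swaps sight checks for a distance check that forgets the player when too far.
; The move macro steers directly with movement input on a clear trace, falling back to AIMoveTo when blocked.
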(event `self.ReceiveBeginPlay`
  (`parent.ReceiveBeginPlay`)
  (`self.Initiation_BotSettings`)
  (`self.StartStop_SightUpdate` true)
  (`self.StartStop_AILogic` true))

(event `Sight`
  (bind _returnvalue (`self.K2_GetActorLocation`))
  (bind _returnvalue_2 (`self.K2_GetActorLocation`))
  (bind _returnvalue_3 (`GameplayStatics.GetPlayerPawn` 0))
  (bind _returnvalue_4 (`self.K2_GetActorLocation` _returnvalue_3))
  (bind _returnvalue_5 (`self.K2_GetActorLocation` _returnvalue_3))
  (bind _returnvalue_6 (`KismetMathLibrary.Dot_VectorVector` (`KismetMathLibrary.Normal` (- _returnvalue_5 _returnvalue)) (`self.GetActorForwardVector`)))
  ;[1 1 1] Перегружаются в дочерних классах
  ;[0 0.2963 1] Sight
  (if (<= (`KismetMathLibrary.Vector_Distance` _returnvalue _returnvalue_5) (`.Sight_Distance_4_D10365ED44F869796F26038B026909D1` (break `/Game/Hell/Core/DATA/Structures/S_AI_Settings` (`self.GetAISettings`))))
    (if (> _returnvalue_6 0.0)
      (if (<= (`KismetMathLibrary.DegAcos` _returnvalue_6) (* (`.Sight_Cone_Degrees_6_A1A5C918477725D6C38735812FFC2DF2` (break `/Game/Hell/Core/DATA/Structures/S_AI_Settings` (`self.GetAISettings`))) 0.5))
        (bind (_outhit _returnvalue_7) (`KismetSystemLibrary.LineTraceSingle` _returnvalue_2 (+ (* (`KismetMathLibrary.Normal` (- _returnvalue_4 _returnvalue_2)) 15.0) _returnvalue_4) "TraceTypeQuery2"))
        (if _returnvalue_7
          (if (== _returnvalue_3 (`.HitActor` (`GameplayStatics.BreakHitResult` _outhit)))
            (`/Game/Hell/Core/Interfaces/BPI_AI.SetPlayerForKnow` _returnvalue_3)))))))

(event `State:None`
  ;[1 1 1] Перегружаются в дочерних классах
)

(event `State:Idle`
  ;[1 1 1] Перегружаются в дочерних классах
)

(event `State:Pursuit`
  ;[1 1 1] Перегружаются в дочерних классах
)

(event `State:Flee`
  ;[1 1 1] Перегружаются в дочерних классах
)

(event `State:Attack`
  ;[1 1 1] Перегружаются в дочерних классах
)

(fn `AI_Logic_Process`
  (switch `/Game/Hell/Core/DATA/ENUMS/E_BotStates` (`self.Get_GeneralState`)
    (:`NewEnumerator0`
      (`self.State:None`))
    (:`NewEnumerator1`
      (`self.State:Idle`))
    (:`NewEnumerator2`
      (`self.State:Pursuit`))
    (:`NewEnumerator3`
      (`self.State:Flee`))
    (:`NewEnumerator4`
      (`self.State:Attack`))))

(fn `FollowPlayerUpdate`
  (bind _foundedplayer (`self.FoundedPlayer`)
    (:`then`
      (if (>= (`KismetMathLibrary.Vector_Distance` (`self.K2_GetActorLocation` _foundedplayer) (`self.K2_GetActorLocation`)) (`.Player_Lost_Distance_11_03EE7F484161F1EB749329989F942609` (break `/Game/Hell/Core/DATA/Structures/S_AI_Settings` (`self.GetAISettings`))))
        (`/Game/Hell/Core/Interfaces/BPI_AI.SetPlayerForKnow` null)))
    (:`else`)))

(fn `Get_GeneralState`
  (returns (AI_General_State :type "/Game/Hell/Core/DATA/ENUMS/E_BotStates Enum"))
  (return (`self.AI_General_State`)))

(fn `GetAISettings`
  (returns (AI_Settings :type "/Game/Hell/Core/DATA/Structures/S_AI_Settings Structure"))
  (return (`self.AI_Settings`)))

(fn `GetIsKnowAboutPlayer`
  (returns (isKnow :type Boolean) (Success :type Boolean))
  (return (`KismetSystemLibrary.IsValid` (`self.FoundedPlayer`)) true))

(fn `Initiation_BotSettings`
  (bind _returnvalue (`|GetDataTableRow` "/Game/Hell/Design/DataTables/AI_Settings.AI_Settings" (`self.Bot'sName`))
    (:`then`
      (set `self.AI_Settings` _returnvalue))))

(fn `OnRep_FoundedPlayer`
  (bind _foundedplayer (`self.FoundedPlayer`))
  (bind _returnvalue (`KismetSystemLibrary.IsValid` _foundedplayer))
  ;[1 1 1] если бот знает об игроке - зрение не обновляется
  (`self.StartStop_SightUpdate` (not _returnvalue))
  ;[1 1 1] Если бот знает об игроке - овключается оценка дистанции до игрока
  (`self.StartStop_FollowUpdate` _returnvalue)
  (`self.Event_FoundedPlayer_Updated` _foundedplayer))

(fn `ResetAllStates`)

(fn `Set_GeneralState`
  (params (AI_General_State :type "/Game/Hell/Core/DATA/ENUMS/E_BotStates Enum" :default "NewEnumerator0"))
  (returns (Success :type Boolean))
  (bind _output_get (set `self.AI_General_State` AI_General_State))
  (`self.ResetAllStates`)
  (`self.Event_GeneralState_Updated` _output_get)
  (return true))

(fn `SetPlayerForKnow`
  (params (PlayersPawn :type "Pawn Object Reference"))
  (returns (Success :type Boolean))
  (set `self.FoundedPlayer` PlayersPawn)
  (return true))

(fn `SetRagdollMode`
  (params (NewValue :type Boolean))
  (returns (Return :type Boolean))
  (bind _output_get (set `self.RagdollMode` NewValue))
  (message `/Game/Hell/Core/Interfaces/BPI_RagdollEffects.RagdollEffect` self NewValue)
  (return _output_get))

(fn `SightUpdate`
  (bind _bp_willcomponent (`self.BP_WillComponent`)
    (:`then`
      (bind (_isdead _success) (`/Game/Hell/Core/ActorComponents/BP_WillComponent.GetIsDead` _bp_willcomponent))
      (if _success
        (if _isdead
          (`self.StartStop_SightUpdate` false :!label _label)
          (else
            (`self.Sight`)))
        (else
          (goto _label))))
    (:`else`
      (goto _label))))

(fn `StartStop_AILogic`
  (params (ToStart :type Boolean :default true))
  (if ToStart
    (bind _returnvalue (`KismetSystemLibrary.K2_SetTimerDelegate` (`|CreateDelegate` :!event `AI_Logic_Process`) (/ 1.0 (`KismetMathLibrary.Conv_IntToDouble` (`GameUserSettings.GetFramePace`))) true))
    (set `self.Timer_AILogic_Process` _returnvalue)
    (else
      (`KismetSystemLibrary.K2_ClearAndInvalidateTimerHandle` (`self.Timer_AILogic_Process`)))))

(fn `StartStop_FollowUpdate`
  (params (toStart :type Boolean :default true))
  (if toStart
    (bind _returnvalue (`KismetSystemLibrary.K2_SetTimerDelegate` (`|CreateDelegate` :!event `FollowPlayerUpdate`) 0.2 true))
    (set `self.Timer_FollowPlayerUpdate` _returnvalue)
    (else
      (`KismetSystemLibrary.K2_ClearAndInvalidateTimerHandle` (`self.Timer_FollowPlayerUpdate`)))))

(fn `StartStop_SightUpdate`
  (params (toStart :type Boolean :default true))
  (if toStart
    (bind _returnvalue (`KismetSystemLibrary.K2_SetTimerDelegate` (`|CreateDelegate` :!event `SightUpdate`) (`self.Rate_SightUpdate`) true))
    (set `self.Timer_SightUpdate` _returnvalue)
    (else
      (`KismetSystemLibrary.K2_ClearAndInvalidateTimerHandle` (`self.Timer_SightUpdate`)))))

(fn `UserConstructionScript`
  (`parent.UserConstructionScript`))