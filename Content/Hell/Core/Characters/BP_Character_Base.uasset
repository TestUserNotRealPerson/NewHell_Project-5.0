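; Base character Blueprint that uses a Will component as its health pool, draining it on damage and freezing the character's time dilation on death.
; Any and Point damage feed one gated handler that blocks further hits for a frame so they don't stack; point hits also call HitEffect.
; Will changes scale the face material's emissive.
; HitEffect, catch and notify functions are stubs, alongside Will and walk-speed helpers.
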(event `self.ReceiveBeginPlay`
  ;[1 0 0.9935] begin play
  (`self.Init_FaceMaterial`)
  (`self.Init_WillComponent`))

(event `self.ReceivePointDamage`
  (params (Damage :type "Float (single-precision)") (DamageType :type "DamageType Object Reference") (HitLocation :type "Vector Structure") (HitNormal :type "Vector Structure") (HitComponent :type "PrimitiveComponent Object Reference") (BoneName :type Name) (ShotFromDirection :type "Vector Structure") (InstigatedBy :type "Controller Object Reference") (DamageCauser :type "Actor Object Reference") (HitInfo :type "HitResult Structure (by ref)"))
  ;[1 0.928 0] damage interface
  (`self.DamageIn` Damage true HitInfo DamageCauser))

(event `self.ReceiveAnyDamage`
  (params (Damage :type "Float (single-precision)") (DamageType :type "DamageType Object Reference") (InstigatedBy :type "Controller Object Reference") (DamageCauser :type "Actor Object Reference"))
  ;[1 0.928 0] damage interface
  (`self.DamageIn` Damage false (struct) DamageCauser))

(event `self.BP_WillComponent.Event_Will_Changed`
  (params (Will :type "Float (single-precision)"))
  ;[1 0.928 0] damage interface
  (`self.Event_OnWillChanged` Will))

(event `DamageIn`
  (params (Damage :type "Float (double-precision)") (UseHitEffect :type Boolean) (HitInfo :type "HitResult Structure") (HitCauser :type "Actor Object Reference"))
  ;[0 1 0.9889] Damage event
  (`|ExecutionSequence`
    (:`then_0`
      (`/Engine/EditorBlueprintResources/StandardMacros.Gate` false :!label _label
        (:`Exit`
          (`/Game/Hell/Core/ActorComponents/BP_WillComponent.IncreaseDecreaseWill_Current` (`self.BP_WillComponent`) false Damage)
          (if UseHitEffect
            (`self.HitEffect` HitInfo HitCauser))
          ;;[1 1 1] задержка нужна для того, чтоб урон из разных источников не суммировался в одном кадре (AnyDamage и PointDamage)
          (`KismetSystemLibrary.Delay` (`GameplayStatics.GetWorldDeltaSeconds`))
          (goto _label :!via `Open`))))
    (:`then_1`
      (goto _label :!via `Close`))))

(fn `Catched`
  (params (Catcher :type "Pawn Object Reference"))
  (returns (Success :type Boolean))
  (return false))

(fn `Decatched`
  (params (Catcher :type "Pawn Object Reference"))
  (returns (Success :type Boolean))
  (return false))

(fn `Event_Dead`
  (set `self.CustomTimeDilation` 0.0))

(fn `Get_Will`
  (returns (Current :type "Float (double-precision)") (Maximum :type "Float (double-precision)") (Success :type Boolean))
  (bind _bp_willcomponent (`self.BP_WillComponent`)
    (:`then`
      (bind (_current _maximum _success) (`/Game/Hell/Core/Interfaces/BPI_Will.Get_Will` _bp_willcomponent))
      (return _current _maximum _success))
    (:`else`
      (return 0.0 0.0 false))))

(fn `GetMaxWalkSpeed`
  (returns (Speed :type "Float (double-precision)") (Success :type Boolean))
  (bind _charactermovement (`self.CharacterMovement`)
    (:`then`
      (return (`CharacterMovementComponent.MaxWalkSpeed` _charactermovement) true))
    (:`else`
      (return 0.0 false))))

(fn `GetNormalizedWalkSpeed`
  (returns (Speed :type "Float (double-precision)") (Success :type Boolean))
  (bind _charactermovement (`self.CharacterMovement`)
    (:`then`
      (return (/ (`KismetMathLibrary.VSize` (`self.GetVelocity`)) (`CharacterMovementComponent.MaxWalkSpeed` _charactermovement)) true))
    (:`else`
      (return 0.0 false))))

(fn `HitEffect`
  (params (HitInfo :type "HitResult Structure") (HitCauser :type "Actor Object Reference")))

(fn `IncreaseDecreaseWill`
  (params (ToIncrease :type Boolean) (Amount :type "Float (double-precision)"))
  (returns (Left :type "Float (double-precision)") (Success :type Boolean))
  (bind (_left _success) (`/Game/Hell/Core/Interfaces/BPI_Will.IncreaseDecreaseWill` (`self.BP_WillComponent`) ToIncrease Amount))
  (return _left _success))

(fn `Init_FaceMaterial`
  (returns (Success :type Boolean))
  (bind _mesh (`self.Mesh`))
  (bind _returnvalue (`PrimitiveComponent.GetMaterial` _mesh 1))
  (`/Engine/EditorBlueprintResources/StandardMacros.IsValid` _returnvalue
    (:`Is Valid`
      (bind _returnvalue_2 (`PrimitiveComponent.CreateDynamicMaterialInstance` _mesh 1 _returnvalue "None"))
      (bind _output_get (set `self.FaceMaterial` _returnvalue_2))
      (bind _returnvalue_3 (`MaterialInstanceDynamic.K2_GetScalarParameterValue` _output_get "Emissive"))
      (set `self.FaceMaterial_StartEmissive` _returnvalue_3)
      (return (`KismetSystemLibrary.IsValid` (`self.FaceMaterial`))))
    (:`Is Not Valid`
      (return false))))

(fn `Init_WillComponent`
  (returns (Success :type Boolean))
  (bind _bp_willcomponent (`self.BP_WillComponent`)
    (:`then`
      (add `/Game/Hell/Core/ActorComponents/BP_WillComponent.Event_Dead` _bp_willcomponent (`|CreateDelegate` :!event `Event_Dead`))
      (add `/Game/Hell/Core/ActorComponents/BP_WillComponent.Event_Will_Changed` _bp_willcomponent (`|CreateDelegate` :!event `OnCurrentWillChanged`))
      (`/Game/Hell/Core/ActorComponents/BP_WillComponent.SetWill_Maximum` _bp_willcomponent (`self.Will_Maximum`))
      (`/Game/Hell/Core/ActorComponents/BP_WillComponent.SetWill_Current` _bp_willcomponent (`self.Will_Current`))
      (return true))
    (:`else`
      (return false))))

(fn `Notify_Attack`
  (returns (Success :type Boolean))
  (return true))

(fn `Notify_Catch`
  (returns (Success :type Boolean))
  (return true))

(fn `OnCurrentWillChanged`
  (params (Will :type "Float (double-precision)"))
  (bind (_will_current _will_maximum) (`/Game/Hell/Core/ActorComponents/BP_WillComponent.GetWill` (`self.BP_WillComponent`)))
  (bind _facematerial (`self.FaceMaterial`)
    (:`then`
      (`MaterialInstanceDynamic.SetScalarParameterValue` _facematerial "Emissive" (* (`self.FaceMaterial_StartEmissive`) (/ _will_current _will_maximum))))
    (:`else`)))

(fn `TryToUseWill`
  (params (Amount :type "Float (double-precision)"))
  (returns (Success :type Boolean))
  (bind _success (`/Game/Hell/Core/Interfaces/BPI_Will.TryToUseWill` (`self.BP_WillComponent`) Amount))
  (return _success))

(fn `UserConstructionScript`)