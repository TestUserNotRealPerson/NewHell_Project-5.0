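; Actor component that stores an actor's Will, a current and maximum pool that works as both a spendable resource and a life value.
; Getters, setters and an increase/decrease function read and write the pool, while TryToUseWill spends only if the remainder stays above zero.
; The RepNotify on current Will clamps it between zero and maximum, fires a change event, and fires a death event near zero.
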(fn `Get_Will`
  (returns (Current :type "Float (double-precision)") (Maximum :type "Float (double-precision)") (Success :type Boolean))
  (bind (_will_current _will_maximum _success) (`self.GetWill`))
  (return _will_current _will_maximum _success))

(fn `GetIsDead`
  (returns (isDead :type Boolean) (Success :type Boolean))
  (return (<= (`self.Will_Current`) 0.0) true))

(fn `GetWill`
  (returns (Will_Current :type "Float (double-precision)") (Will_Maximum :type "Float (double-precision)") (Success :type Boolean))
  (return (`self.Will_Current`) (`self.Will_Maximum`) true))

(fn `GetWill_Enough`
  (params (Value :type "Float (double-precision)"))
  (returns (IsEnough :type Boolean) (Success :type Boolean))
  (return (<= Value (`self.Will_Current`)) true))

(fn `IncreaseDecreaseWill`
  (params (ToIncrease :type Boolean) (Amount :type "Float (double-precision)"))
  (returns (Left :type "Float (double-precision)") (Success :type Boolean))
  (bind (_left _success) (`self.IncreaseDecreaseWill_Current` ToIncrease Amount))
  (return _left _success))

(fn `IncreaseDecreaseWill_Current`
  (params (ToIncrease :type Boolean :default true) (Amount :type "Float (double-precision)"))
  (returns (Left :type "Float (double-precision)") (Success :type Boolean))
  (bind _output_get (set `self.Will_Current` (+ (`self.Will_Current`) (* (`KismetMathLibrary.SelectFloat` 1.0 -1.0 ToIncrease) (`KismetMathLibrary.Abs` Amount)))))
  (return _output_get true))

(fn `OnRep_Will_Current`
  (bind _will_maximum (`self.Will_Maximum`))
  (bind _will_current (`self.Will_Current`))
  (`|ExecutionSequence`
    (:`then_0`
      ;[1 1 1] выравнивание переменной в рамки минмакс
      (if (or (< _will_current 0.0) (> _will_current _will_maximum))
        (set `self.Will_Current` (`KismetMathLibrary.FClamp` _will_current 0.0 _will_maximum)))
      (`self.Event_Will_Changed` (`self.Will_Current`)))
    (:`then_1`
      ;[1 1 1] эвент смерти
      (if (`KismetMathLibrary.NearlyEqual_FloatFloat` _will_current)
        (`self.Event_Dead`)))))

(fn `SetWill_Current`
  (params (Will_Current :type "Float (double-precision)"))
  (set `self.Will_Current` Will_Current))

(fn `SetWill_Maximum`
  (params (Will_Current :type "Float (double-precision)"))
  (set `self.Will_Maximum` Will_Current))

(fn `TryToUseWill`
  (params (Amount :type "Float (double-precision)"))
  (returns (Success :type Boolean))
  (if (> (- (`self.GetWill`) Amount) 0.0)
    (`self.IncreaseDecreaseWill_Current` false Amount)
    (return true)
    (else
      (return false))))