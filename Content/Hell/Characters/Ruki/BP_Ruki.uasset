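; Ruki is an enemy AI character that hunts the player, grabs them and damages them while held.
; Player awareness, distance and a Will threshold drive its idle, pursuit and attack states.
; The catch notify sphere-traces from a hand socket; the CatchedActor OnRep then attaches and lerps the victim there, and damage feeds Will back.
; Hits play directional montages, and bumping a ragdolled Relo or Ruki costs both characters Will.
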(event `self.ReceiveBeginPlay`
  (`parent.ReceiveBeginPlay`)
  (add `self.Event_FoundedPlayer_Updated` (`|CreateDelegate` :!event `ChangePlayerStatus`))
  (add `self.Event_GeneralState_Updated` (`|CreateDelegate` :!event `ChangeGeneralStatus`)))

(event `self.BP_WillComponent.Event_Will_Changed`
  (params (Will :type "Float (single-precision)"))
  (bind (_isknow _success) (`/Game/Hell/Core/Interfaces/BPI_AI.GetIsKnowAboutPlayer`))
  (if _success
    (if _isknow
      (`self.Catched_Actor`
        (:`then`)
        (:`else`
          (`self.Set_GeneralState` (select `bool` (> (`/Game/Hell/Core/ActorComponents/BP_WillComponent.GetWill` (`self.BP_WillComponent`)) 100.0) :`false` "NewEnumerator2" :`true` "NewEnumerator1" :!type "/Game/Hell/Core/DATA/ENUMS/E_BotStates Enum"))))
      (else
        (`self.Set_GeneralState` "NewEnumerator1" :!label _label)))
    (else
      (goto _label))))

(event `ChangePlayerStatus` :!signature `self.Event_FoundedPlayer_Updated`
  (params (Player :type "Pawn Object Reference"))
  ;[1 1 1] последствия изменения статуса видимого игрока
  (`/Engine/EditorBlueprintResources/StandardMacros.IsValid` Player
    (:`Is Valid`
      (`self.Set_GeneralState` (select `bool` (> (`/Game/Hell/Core/ActorComponents/BP_WillComponent.GetWill` (`self.BP_WillComponent`)) 100.0) :`false` "NewEnumerator2" :`true` "NewEnumerator1" :!type "/Game/Hell/Core/DATA/ENUMS/E_BotStates Enum")))
    (:`Is Not Valid`
      (`self.Set_GeneralState` "NewEnumerator1"))))

(event `CatchDecatch_Behavior`
  (params (isCatch :type Boolean :default true))
  (bind _catched_actor (`self.Catched_Actor`))
  (bind _mesh (`self.Mesh`))
  ;[1 1 1] функции поведения, когда есть пойманный игрок, и когда его нет
  (if isCatch
    (`self.K2_AttachToComponent` _catched_actor _mesh "SCK_Catcher" "KeepWorld" "KeepWorld" "KeepWorld" true)
    (bind (_direction _alpha) (`Timeline|Catching` :!via `PlayFromStart`)
      (:`Update`
        (`self.K2_SetActorLocation` _catched_actor (`KismetMathLibrary.VLerp` (`self.K2_GetActorLocation` _catched_actor) (`SceneComponent.GetSocketLocation` _mesh "SCK_Catcher") _alpha) false false))
      (:`Finished`
        (`self.Set_GeneralState` "NewEnumerator0")))
    (else
      (`self.Set_GeneralState` "NewEnumerator1")
      (`|PlayMontage` null "/Game/Hell/Assets/Ruki/Animations/rukiidle_Anim_skelet_de_catching_Montage.rukiidle_Anim_skelet_de_catching_Montage"))))

(event `self.State:Idle`
  (bind _returnvalue (`self.K2_GetActorLocation`))
  (bind ((`Sight_Distance_4_D10365ED44F869796F26038B026909D1` _sight_distance)) (break `/Game/Hell/Core/DATA/Structures/S_AI_Settings` (`self.GetAISettings`)))
  (bind _returnvalue_2 (`self.K2_GetActorLocation` (`GameplayStatics.GetPlayerPawn` 0)))
  (bind _returnvalue_3 (`KismetMathLibrary.Dot_VectorVector` (`KismetMathLibrary.Normal` (- _returnvalue_2 _returnvalue)) (`self.GetActorForwardVector`)))
  ;[0 1 0.9913] IDLE
  (bind (_isknow _success) (`/Game/Hell/Core/Interfaces/BPI_AI.GetIsKnowAboutPlayer`))
  (if _success
    (if _isknow
      (if (<= (`KismetMathLibrary.Vector_Distance` _returnvalue_2 _returnvalue) (`.Attack_Distance_2_B8B2ED334AEB90E742D8BEAB441EE22E` (break `/Game/Hell/Core/DATA/Structures/S_AI_Settings` (`self.GetAISettings`))))
        (if (>= _returnvalue_3 0.0)
          (if (`KismetMathLibrary.NearlyEqual_FloatFloat` _sight_distance 180.0 0.001)
            (`self.Set_GeneralState` "NewEnumerator4" :!label _label)
            (elif (>= (* _sight_distance 0.5) (`KismetMathLibrary.DegAcos` _returnvalue_3))
              (goto _label))))))))

(event `self.State:Pursuit`
  ;[0 1 0.9913] Pursuit
  (if (<= (`KismetMathLibrary.Vector_Distance` (`self.K2_GetActorLocation` (`GameplayStatics.GetPlayerPawn` 0)) (`self.K2_GetActorLocation`)) (`.Attack_Distance_2_B8B2ED334AEB90E742D8BEAB441EE22E` (break `/Game/Hell/Core/DATA/Structures/S_AI_Settings` (`self.GetAISettings`))))
    (`self.Set_GeneralState` "NewEnumerator4")
    (else
      (`|AIMoveTo` self (`self.K2_GetActorLocation` (`GameplayStatics.GetPlayerPawn` 0)) null))))

(event `ChangeGeneralStatus`
  (params (State :type "/Game/Hell/Core/DATA/ENUMS/E_BotStates Enum" :default "NewEnumerator0")))

(event `self.ReceiveTick`
  (params (DeltaSeconds :type "Float (single-precision)"))
  ;[1 0 0.05869 1 30] TICK
)

(event `self.State:Attack`
  (bind (_returnvalue_roll _returnvalue_pitch) (`KismetMathLibrary.BreakRotator` (`self.K2_GetActorRotation`)))
  (bind _mesh (`self.Mesh`))
  (bind (_returnvalue_roll_2 _returnvalue_pitch_2 _returnvalue_yaw) (`KismetMathLibrary.BreakRotator` (`KismetMathLibrary.FindLookAtRotation` (`self.K2_GetActorLocation`) (`self.K2_GetActorLocation` (`GameplayStatics.GetPlayerPawn` 0)))))
  ;[0 1 0.9913] Attack
  (if (<= (`KismetMathLibrary.Vector_Distance` (`self.K2_GetActorLocation` (`GameplayStatics.GetPlayerPawn` 0)) (`self.K2_GetActorLocation`)) (`.Attack_Distance_2_B8B2ED334AEB90E742D8BEAB441EE22E` (break `/Game/Hell/Core/DATA/Structures/S_AI_Settings` (`self.GetAISettings`))))
    (`self.K2_SetActorRotation` (`KismetMathLibrary.MakeRotator` _returnvalue_roll _returnvalue_pitch _returnvalue_yaw))
    (if (not (`AnimInstance.IsAnyMontagePlaying` (`SkeletalMeshComponent.GetAnimInstance` _mesh)))
      (`|PlayMontage` _mesh "/Game/Hell/Assets/Ruki/Animations/rukiidle_Anim_skelet_catching_Montage.rukiidle_Anim_skelet_catching_Montage" 1.0 0.0 "None"))
    (else
      (`self.Set_GeneralState` (select `bool` (> (`/Game/Hell/Core/ActorComponents/BP_WillComponent.GetWill` (`self.BP_WillComponent`)) 100.0) :`false` "NewEnumerator2" :`true` "NewEnumerator1" :!type "/Game/Hell/Core/DATA/ENUMS/E_BotStates Enum")))))

(event `self.State:None`
  (bind ((`Main_Attack_Damage_14_FEA9B05746B12381244B538F3848CF53` _main_attack_damage) (`Main_Skill_WillFeedback_16_894274644053CF139CC1D19C110866B8` _main_skill_willfeedback)) (break `/Game/Hell/Core/DATA/Structures/S_AI_Settings` (`self.GetAISettings`)))
  ;[0 1 0.9913] State:None используется во время Catching'a
  (bind _catched_actor (`self.Catched_Actor`)
    (:`then`
      (`KismetSystemLibrary.Delay` 1.0)
      (`GameplayStatics.ApplyDamage` _catched_actor _main_attack_damage (`self.GetController`) self)
      (`self.IncreaseDecreaseWill` true _main_skill_willfeedback))
    (:`else`
      (`self.Set_GeneralState` "NewEnumerator1"))))

(event `self.CapsuleComponent.OnComponentHit`
  (params (HitComponent :type "PrimitiveComponent Object Reference") (OtherActor :type "Actor Object Reference") (OtherComp :type "PrimitiveComponent Object Reference") (NormalImpulse :type "Vector Structure") (Hit :type "HitResult Structure (by ref)"))
  (bind _returnvalue (`GameplayStatics.GetObjectClass` OtherActor))
  (bind _capsulecomponent (`self.CapsuleComponent`))
  (bind (_returnvalue_roll _returnvalue_pitch _returnvalue_yaw) (`KismetMathLibrary.BreakRotator` (`SceneComponent.K2_GetComponentRotation` _capsulecomponent)))
  (if (and (or (== _returnvalue "/Game/Hell/Characters/Relo/BP_Relo.BP_Relo_C") (== _returnvalue "BP_Ruki_C")) (not (`self.InDelay`)))
    (bind _output_get (set `self.HitedActor` OtherActor))
    (bind _asbp_character_base_ai (cast `/Game/Hell/Core/Characters/BP_Character_Base_AI` _output_get))
    (if (`/Game/Hell/Core/Characters/BP_Character_Base_AI.RagdollMode` _asbp_character_base_ai)
      (bind (_returnvalue_roll_2 _returnvalue_pitch_2 _returnvalue_yaw_2) (`KismetMathLibrary.BreakRotator` (`KismetMathLibrary.FindLookAtRotation` (`SceneComponent.K2_GetComponentLocation` _capsulecomponent) (`SceneComponent.K2_GetComponentLocation` (`Character.CapsuleComponent` _asbp_character_base_ai)))))
      (bind _returnvalue_2 (`KismetMathLibrary.NormalizeAxis` (- _returnvalue_yaw _returnvalue_yaw_2)))
      (`KismetSystemLibrary.PrintString` (`KismetStringLibrary.Conv_DoubleToString` _returnvalue_2) true true (struct :`R` 1.0 :`G` 0.059748 :`B` 0.019947 :`A` 1.0) 30.0)
      (set `self.InDelay` true)
      (if (and (> _returnvalue_2 -90.0) (< _returnvalue_2 90.0))
        (`|PlayMontage` (`self.Mesh`) "/Game/Hell/Assets/Ruki/Animations/rukiidle_Anim_skelet_attack_taking_front_run_Montage.rukiidle_Anim_skelet_attack_taking_front_run_Montage"
          (:`then`
            (`KismetSystemLibrary.Delay` 1.0)
            (set `self.InDelay` false)))
        (else
          (`|PlayMontage` null "/Game/Hell/Assets/Ruki/Animations/rukiidle_Anim_skelet_attack_taking_back_stay_Montage.rukiidle_Anim_skelet_attack_taking_back_stay_Montage"
            (:`then`
              (`KismetSystemLibrary.Delay` 1.0)
              (set `self.InDelay` false)))))
      (`self.IncreaseDecreaseWill` false 20.0)
      (message `/Game/Hell/Core/Interfaces/BPI_Will.IncreaseDecreaseWill` (`self.HitedActor`) false 10.0))))

(fn `Decatched`
  (params (Catcher :type "Pawn Object Reference"))
  (returns (Success :type Boolean))
  (bind _catched_actor (`self.Catched_Actor`)
    (:`then`
      (set `self.Catched_Actor` null))
    (:`else`
      _))
  (return (not (`KismetSystemLibrary.IsValid` _catched_actor))))

(fn `Get_GeneralState`
  (returns (AI_General_State :type "/Game/Hell/Core/DATA/ENUMS/E_BotStates Enum"))
  (return (`parent.Get_GeneralState`)))

(fn `HitEffect`
  (params (HitInfo :type "HitResult Structure") (HitCauser :type "Actor Object Reference"))
  (bind (_returnvalue_x _returnvalue_y) (`KismetMathLibrary.BreakVector` (`self.GetVelocity`)))
  (bind _returnvalue (`KismetMathLibrary.Normal` (- (`self.K2_GetActorLocation` HitCauser) (`self.K2_GetActorLocation`))))
  (bind _side (`/Game/Hell/Core/FunctionLibraries/BPFL_General.Convert_Dots_To_Side` (`KismetMathLibrary.Dot_VectorVector` (`self.GetActorForwardVector`) _returnvalue) (`KismetMathLibrary.Dot_VectorVector` _returnvalue (`self.GetActorRightVector`))))
  (`parent.HitEffect` HitInfo HitCauser)
  (`self.PlayAnimMontage` (select `bool` (> (`KismetMathLibrary.VSize` (`KismetMathLibrary.MakeVector` _returnvalue_x _returnvalue_y)) 5.0) :`false` (select `/Game/Hell/Core/DATA/ENUMS/E_Sides` _side :`NewEnumerator0` "/Game/Hell/Assets/Ruki/Animations/rukiidle_Anim_skelet_attack_taking_front_stay_Montage.rukiidle_Anim_skelet_attack_taking_front_stay_Montage" :`NewEnumerator2` "/Game/Hell/Assets/Ruki/Animations/rukiidle_Anim_skelet_attack_taking_back_stay_Montage.rukiidle_Anim_skelet_attack_taking_back_stay_Montage" :`NewEnumerator3` "/Game/Hell/Assets/Ruki/Animations/rukiidle_Anim_skelet_attack_taking_right_stay_Montage.rukiidle_Anim_skelet_attack_taking_right_stay_Montage" :`NewEnumerator4` "/Game/Hell/Assets/Ruki/Animations/rukiidle_Anim_skelet_attack_taking_left_stay_Montage.rukiidle_Anim_skelet_attack_taking_left_stay_Montage" :!type "AnimMontage Object Reference") :`true` (select `/Game/Hell/Core/DATA/ENUMS/E_Sides` _side :`NewEnumerator0` "/Game/Hell/Assets/Ruki/Animations/rukiidle_Anim_skelet_attack_taking_front_run_Montage.rukiidle_Anim_skelet_attack_taking_front_run_Montage" :`NewEnumerator2` "/Game/Hell/Assets/Ruki/Animations/rukiidle_Anim_skelet_attack_taking_back_run_Montage.rukiidle_Anim_skelet_attack_taking_back_run_Montage" :`NewEnumerator3` "/Game/Hell/Assets/Ruki/Animations/rukiidle_Anim_skelet_attack_taking_right_run_Montage.rukiidle_Anim_skelet_attack_taking_right_run_Montage" :`NewEnumerator4` "/Game/Hell/Assets/Ruki/Animations/rukiidle_Anim_skelet_attack_taking_left_run_Montage.rukiidle_Anim_skelet_attack_taking_left_run_Montage" :!type "AnimMontage Object Reference"))))

(fn `Notify_Catch`
  (returns (Success :type Boolean))
  (bind _mesh (`self.Mesh`))
  (bind _returnvalue (`SceneComponent.GetSocketLocation` _mesh "SCK_Catcher"))
  (bind _success (`parent.Notify_Catch`))
  (if _success
    (bind _outhits (`KismetSystemLibrary.SphereTraceMulti` :`Start` _returnvalue :`End` (+ _returnvalue (* (`SceneComponent.GetRightVector` _mesh) 5.0)) :`Radius` 15.0 :`TraceChannel` "TraceTypeQuery2" :`bTraceComplex` true :`DrawTime` 1.0))
    (for _array_element _outhits
      (bind _asbp_character_base (cast `/Game/Hell/Core/Characters/BP_Character_Base` (`.HitActor` (`GameplayStatics.BreakHitResult` _array_element))))
      (if (`self.IsPlayerControlled` _asbp_character_base)
        (bind _output_get (set `self.Catched_Actor` _asbp_character_base))
        (`/Game/Hell/Core/Interfaces/BPI_SkillEffects.Catched` _output_get self)
        (break)))
    (return true)
    (else
      (return false))))

(fn `OnRep_Catched_Actor`
  (`self.CatchDecatch_Behavior` (`KismetSystemLibrary.IsValid` (`self.Catched_Actor`))))

(fn `RagdollEffect`
  (params (`On/Off` :type Boolean))
  (returns (Return :type Boolean))
  (return `On/Off`))

(fn `Set_GeneralState`
  (params (AI_General_State :type "/Game/Hell/Core/DATA/ENUMS/E_BotStates Enum" :default "NewEnumerator0"))
  (returns (Success :type Boolean))
  (bind _success (`parent.Set_GeneralState` AI_General_State))
  (return _success))

(fn `UserConstructionScript`
  (`parent.UserConstructionScript`))