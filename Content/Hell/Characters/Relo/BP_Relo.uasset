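; Relo enemy AI character that wanders when idle and, once aware of the player, pursues or flees depending on its Will ratio.
; A state machine drives movement, using gated random navmesh points for wandering and fleeing, and AIMoveTo for pursuit.
; Montage-driven melee sphere-traces from the right hand to damage and push the player, restoring Will.
; Colliding with a ragdolled Relo or Ruki triggers directional hit montages and drains both characters' Will.
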(event `self.ReceiveBeginPlay`
  (`parent.ReceiveBeginPlay`)
  (add `self.Event_FoundedPlayer_Updated` (`|CreateDelegate` :!event `ChangePlayerStatus`))
  (add `self.Event_GeneralState_Updated` (`|CreateDelegate` :!event `ChangeGeneralStatus`)))

(event `self.BP_WillComponent.Event_Will_Changed`
  (params (Will :type "Float (single-precision)"))
  (bind (_will_current _will_maximum) (`/Game/Hell/Core/ActorComponents/BP_WillComponent.GetWill` (`self.BP_WillComponent`)))
  (if (not (`self.RagdollMode`))
    (bind (_isknow _success) (`/Game/Hell/Core/Interfaces/BPI_AI.GetIsKnowAboutPlayer`))
    (if _success
      (if _isknow
        (`self.Set_GeneralState` (select `bool` (> (/ _will_current _will_maximum) 0.5) :`false` "NewEnumerator3" :`true` "NewEnumerator2" :!type "/Game/Hell/Core/DATA/ENUMS/E_BotStates Enum"))
        (else
          (`self.Set_GeneralState` "NewEnumerator1" :!label _label)))
      (else
        (goto _label)))))

(event `ChangePlayerStatus` :!signature `self.Event_FoundedPlayer_Updated`
  (params (Player :type "Pawn Object Reference"))
  (bind (_will_current _will_maximum) (`/Game/Hell/Core/ActorComponents/BP_WillComponent.GetWill` (`self.BP_WillComponent`)))
  (if (not (`self.RagdollMode`))
    (`/Engine/EditorBlueprintResources/StandardMacros.IsValid` Player
      (:`Is Valid`
        (`self.Set_GeneralState` (select `bool` (> (/ _will_current _will_maximum) 0.5) :`false` "NewEnumerator3" :`true` "NewEnumerator2" :!type "/Game/Hell/Core/DATA/ENUMS/E_BotStates Enum")))
      (:`Is Not Valid`
        (`self.Set_GeneralState` "NewEnumerator1")))))

(event `self.ReceiveAnyDamage`
  (params (Damage :type "Float (single-precision)") (DamageType :type "DamageType Object Reference") (InstigatedBy :type "Controller Object Reference") (DamageCauser :type "Actor Object Reference"))
  (`parent.ReceiveAnyDamage` Damage DamageType InstigatedBy DamageCauser)
  (if (`Controller.IsPlayerController` InstigatedBy)
    (`/Game/Hell/Core/Interfaces/BPI_AI.SetPlayerForKnow` (`Controller.K2_GetPawn` InstigatedBy))))

(event `RagdollIn`
  (params (`On/Off` :type Boolean))
  (`KismetSystemLibrary.PrintString` (`KismetStringLibrary.Conv_BoolToString` (`self.RagdollMode`)))
  (if `On/Off`
    (`CharacterMovementComponent.DisableMovement` (`self.CharacterMovement`))
    (`PrimitiveComponent.SetCollisionEnabled` (`self.Mesh`) "QueryAndPhysics")
    (else
      (bind (_current _maximum) (`self.Get_Will`))
      (if (`self.Alive`)
        _))))

(event `self.CapsuleComponent.OnComponentHit`
  (params (HitComponent :type "PrimitiveComponent Object Reference") (OtherActor :type "Actor Object Reference") (OtherComp :type "PrimitiveComponent Object Reference") (NormalImpulse :type "Vector Structure") (Hit :type "HitResult Structure (by ref)"))
  (bind _returnvalue (`GameplayStatics.GetObjectClass` OtherActor))
  (bind _mesh (`self.Mesh`))
  (bind _capsulecomponent (`self.CapsuleComponent`))
  (bind (_returnvalue_roll _returnvalue_pitch _returnvalue_yaw) (`KismetMathLibrary.BreakRotator` (`SceneComponent.K2_GetComponentRotation` _capsulecomponent)))
  (if Hit_bBlockingHit
    (if (and (or (== _returnvalue "BP_Relo_C") (== _returnvalue "/Game/Hell/Characters/Ruki/BP_Ruki.BP_Ruki_C")) (not (`self.InDelay`)))
      (bind _output_get (set `self.HitedActor` OtherActor))
      (bind _asbp_character_base_ai (cast `/Game/Hell/Core/Characters/BP_Character_Base_AI` _output_get))
      (if (`/Game/Hell/Core/Characters/BP_Character_Base_AI.RagdollMode` _asbp_character_base_ai)
        (bind (_returnvalue_roll_2 _returnvalue_pitch_2 _returnvalue_yaw_2) (`KismetMathLibrary.BreakRotator` (`KismetMathLibrary.FindLookAtRotation` (`SceneComponent.K2_GetComponentLocation` _capsulecomponent) (`SceneComponent.K2_GetComponentLocation` (`Character.Mesh` _asbp_character_base_ai)))))
        (bind _returnvalue_2 (`KismetMathLibrary.NormalizeAxis` (+ _returnvalue_yaw_2 _returnvalue_yaw)))
        (`KismetSystemLibrary.PrintString` (`KismetStringLibrary.Conv_DoubleToString` _returnvalue_2) true true (struct :`R` 1.0 :`G` 0.059748 :`B` 0.019947 :`A` 1.0) 30.0)
        (set `self.InDelay` true)
        (if (and (> _returnvalue_2 0.0) (< _returnvalue_2 180.0))
          (`|PlayMontage` _mesh "/Game/Hell/Assets/Relo/Animations/relo-npc_Anim_skeletonreuleaux_action_attack_taking___Montage.relo-npc_Anim_skeletonreuleaux_action_attack_taking___Montage"
            (:`then`
              _))
          (elif (and (> _returnvalue_2 -90.0) (< _returnvalue_2 0.0))
            (`|PlayMontage` _mesh "/Game/Hell/Assets/Relo/Animations/relo-npc_Anim_skeletonreuleaux_telekinesis_taking_right_Montage.relo-npc_Anim_skeletonreuleaux_telekinesis_taking_right_Montage"
              (:`then`
                _))
            (else
              (`|PlayMontage` _mesh "/Game/Hell/Assets/Relo/Animations/relo-npc_Anim_skeletonreuleaux_telekinesis_taking_left_Montage.relo-npc_Anim_skeletonreuleaux_telekinesis_taking_left_Montage"
                (:`then`
                  _)))))
        (`KismetSystemLibrary.Delay` 1.0)
        (set `self.InDelay` false)
        (`self.IncreaseDecreaseWill` false 20.0)
        (bind _left (message `/Game/Hell/Core/Interfaces/BPI_Will.IncreaseDecreaseWill` (`self.HitedActor`) false 10.0))
        (if (<= _left 0.0)
          (bind _asbp_romb (cast `/Game/Hell/Characters/Romb/BP_Romb` (`GameplayStatics.GetPlayerPawn` 0)))
          (`/Game/Hell/Characters/Romb/BP_Romb.OutOfRagdollKinesis` _asbp_romb))))))

(event `self.Mesh.OnComponentHit`
  (params (HitComponent :type "PrimitiveComponent Object Reference") (OtherActor :type "Actor Object Reference") (OtherComp :type "PrimitiveComponent Object Reference") (NormalImpulse :type "Vector Structure") (Hit :type "HitResult Structure (by ref)")))

(event `self.ReceiveTick`
  (params (DeltaSeconds :type "Float (single-precision)"))
  ;[1 0 0.05869 1 30] TICK
)

(event `self.State:Idle`
  (bind _returnvalue (`self.K2_GetActorLocation`))
  (bind _destinationpoint (`self.DestinationPoint`))
  ;[0 1 0.9913] IDLE
  (if (not (`self.RagdollMode`))
    (`|ExecutionSequence`
      (:`then_0`
        (`/Engine/EditorBlueprintResources/StandardMacros.Gate` false :!label _label
          (:`Exit`
            (set `self.DestinationPoint` (`KismetMathLibrary.MakeVector` (.x (`NavigationSystemV1.K2_GetRandomLocationInNavigableRadius` (`self.K2_GetActorLocation`) 250.0 null null)) (.y (`NavigationSystemV1.K2_GetRandomLocationInNavigableRadius` (`self.K2_GetActorLocation`) 250.0 null null)) (+ (.z (`NavigationSystemV1.K2_GetRandomLocationInNavigableRadius` (`self.K2_GetActorLocation`) 250.0 null null)) 25.0))))))
      (:`then_1`
        (goto _label :!via `Close`))
      (:`then_2`
        ;;[1 1 1] для айдл режима (считай, для большинства ботов) линейное движение, для оптимизации
        (`self.AddMovementInput` (`KismetMathLibrary.Normal` (- _destinationpoint _returnvalue)))
        (if (<= (`KismetMathLibrary.Vector_Distance` _destinationpoint _returnvalue) (`.Attack_Distance_2_B8B2ED334AEB90E742D8BEAB441EE22E` (break `/Game/Hell/Core/DATA/Structures/S_AI_Settings` (`self.GetAISettings`))))
          ;;[1 1 1] когда точка достигнута, либо не достигнута, бот отдыхает заданное здесь время
          (`KismetSystemLibrary.Delay` (`KismetMathLibrary.RandomFloatInRange` 1.5 3.0))
          (`self.Idle:GenerateNewDesPoint`))))))

(event `Idle:GenerateNewDesPoint`
  ;[0 1 0.9913] IDLE
  (goto _label :!via `Open`))

(event `ChangeGeneralStatus`
  (params (State :type "/Game/Hell/Core/DATA/ENUMS/E_BotStates Enum" :default "NewEnumerator0"))
  (`self.ResetAllStates`))

(event `self.State:Pursuit`
  (bind _returnvalue (`self.K2_GetActorLocation` (`GameplayStatics.GetPlayerPawn` 0)))
  ;[0 1 0.9913] Pursuit
  (if (not (`self.RagdollMode`))
    (`|AIMoveTo` self _returnvalue null
      (:`OnSuccess`
        _)
      (:`OnFail`
        _))
    (if (<= (`KismetMathLibrary.Vector_Distance` _returnvalue (`self.K2_GetActorLocation`)) (`.Attack_Distance_2_B8B2ED334AEB90E742D8BEAB441EE22E` (break `/Game/Hell/Core/DATA/Structures/S_AI_Settings` (`self.GetAISettings`))))
      (`self.Set_GeneralState` "NewEnumerator4"))))

(event `self.State:Flee`
  (bind _returnvalue (`self.K2_GetActorLocation`))
  (bind _returnvalue_2 (`self.K2_GetActorLocation`))
  (bind _destinationpoint (`self.DestinationPoint`))
  ;[0 1 0.9913] Flee
  (`|ExecutionSequence`
    (:`then_0`
      (`/Engine/EditorBlueprintResources/StandardMacros.Gate` false :!label _label_2
        (:`Exit`
          (set `self.DestinationPoint` (`KismetMathLibrary.MakeVector` (.x (`NavigationSystemV1.K2_GetRandomLocationInNavigableRadius` (`self.K2_GetActorLocation`) 250.0 null null)) (.y (`NavigationSystemV1.K2_GetRandomLocationInNavigableRadius` (`self.K2_GetActorLocation`) 250.0 null null)) (+ (.z (`NavigationSystemV1.K2_GetRandomLocationInNavigableRadius` (`self.K2_GetActorLocation`) 250.0 null null)) 25.0)) :!label _label_3)
          (if (>= (`KismetMathLibrary.Dot_VectorVector` (`KismetMathLibrary.Normal` (- _returnvalue_2 (`self.K2_GetActorLocation` (`GameplayStatics.GetPlayerPawn` 0)))) (`KismetMathLibrary.Normal` (- (`self.DestinationPoint`) _returnvalue_2))) 0.5)
            (`self.Flee_Start`)
            (else
              (goto _label_3))))))
    (:`then_1`
      (goto _label_2 :!via `Close`))
    (:`then_2`
      (`/Engine/EditorBlueprintResources/StandardMacros.Gate` true :!label _label_4
        (:`Exit`
          (`self.AddMovementInput` (`KismetMathLibrary.Normal` (- _destinationpoint _returnvalue)))
          (if (<= (`KismetMathLibrary.Vector_Distance` _destinationpoint _returnvalue) (`.Attack_Distance_2_B8B2ED334AEB90E742D8BEAB441EE22E` (break `/Game/Hell/Core/DATA/Structures/S_AI_Settings` (`self.GetAISettings`))))
            (`self.Flee_Stop`)
            (`KismetSystemLibrary.PrintString` "stop")))))))

(event `Flee_Stop`
  ;[0 1 0.9913] Flee
  (`|ExecutionSequence`
    (:`then_0`
      (goto _label_2 :!via `Open`))
    (:`then_1`
      (goto _label_4 :!via `Close`))))

(event `Flee_Start`
  ;[0 1 0.9913] Flee
  (`KismetSystemLibrary.PrintString` "flee")
  (goto _label_4 :!via `Open`))

(event `self.State:Attack`
  (bind _mesh (`self.Mesh`))
  (bind (_will_current _will_maximum) (`/Game/Hell/Core/ActorComponents/BP_WillComponent.GetWill` (`self.BP_WillComponent`)))
  (bind (_returnvalue_roll _returnvalue_pitch _returnvalue_yaw) (`KismetMathLibrary.BreakRotator` (`KismetMathLibrary.FindLookAtRotation` (`self.K2_GetActorLocation`) (`self.K2_GetActorLocation` (`GameplayStatics.GetPlayerPawn` 0)))))
  (bind _returnvalue (`AnimInstance.IsAnyMontagePlaying` (`SkeletalMeshComponent.GetAnimInstance` _mesh)))
  ;[0 1 0.9913] Attack
  (if (`self.RagdollMode`)
    _
    (elif (<= (`KismetMathLibrary.Vector_Distance` (`self.K2_GetActorLocation` (`GameplayStatics.GetPlayerPawn` 0)) (`self.K2_GetActorLocation`)) (`.Attack_Distance_2_B8B2ED334AEB90E742D8BEAB441EE22E` (break `/Game/Hell/Core/DATA/Structures/S_AI_Settings` (`self.GetAISettings`))))
      (`self.K2_SetActorRotation` (`KismetMathLibrary.MakeRotator` 0.0 0.0 _returnvalue_yaw))
      (if (not _returnvalue)
        (`|PlayMontage` _mesh "/Game/Hell/Assets/Relo/Animations/relo-npc_Anim_skeletonreuleaux_action_attack_Montage.relo-npc_Anim_skeletonreuleaux_action_attack_Montage" 1.0 0.0 "None"))
      (elif (not _returnvalue)
        (`self.Set_GeneralState` (select `bool` (> (/ _will_current _will_maximum) 0.5) :`false` "NewEnumerator3" :`true` "NewEnumerator2" :!type "/Game/Hell/Core/DATA/ENUMS/E_BotStates Enum"))))))

(event `Die`
  (set `self.CustomTimeDilation` 0.0))

(fn `AngleCheck`
  (params (Actor :type "Actor Object Reference"))
  (returns (Angle :type "Float (double-precision)"))
  (bind _capsulecomponent (`self.CapsuleComponent`))
  (return (`KismetMathLibrary.DegAcos` (`KismetMathLibrary.Dot_VectorVector` (`KismetMathLibrary.Normal` (- (`self.K2_GetActorLocation` Actor) (`SceneComponent.K2_GetComponentLocation` _capsulecomponent))) (`SceneComponent.GetForwardVector` _capsulecomponent)))))

(fn `Get_GeneralState`
  (returns (AI_General_State :type "/Game/Hell/Core/DATA/ENUMS/E_BotStates Enum"))
  (return (`parent.Get_GeneralState`)))

(fn `Get_Will`
  (returns (Current :type "Float (double-precision)") (Maximum :type "Float (double-precision)") (Success :type Boolean))
  (return 1.0 10.0 true))

(fn `HitEffect`
  (params (HitInfo :type "HitResult Structure") (HitCauser :type "Actor Object Reference"))
  (bind _returnvalue (`KismetMathLibrary.Dot_VectorVector` (`.ImpactNormal` (`GameplayStatics.BreakHitResult` HitInfo)) (`KismetMathLibrary.Normal` (`SceneComponent.GetForwardVector` (`self.Mesh`)))))
  (bind _returnvalue_2 (and (>= _returnvalue 0.5) (<= _returnvalue 0.9)))
  (`parent.HitEffect` HitInfo null)
  (`self.PlayAnimMontage` (select `bool` (xor (and (<= _returnvalue -0.5) (>= _returnvalue -0.9)) _returnvalue_2) :`false` "/Game/Hell/Assets/Relo/Animations/relo-npc_Anim_skeletonreuleaux_action_attack_taking___Montage.relo-npc_Anim_skeletonreuleaux_action_attack_taking___Montage" :`true` (select `bool` _returnvalue_2 :`false` "/Game/Hell/Assets/Relo/Animations/relo-npc_Anim_skeletonreuleaux_telekinesis_taking_left_Montage.relo-npc_Anim_skeletonreuleaux_telekinesis_taking_left_Montage" :`true` "/Game/Hell/Assets/Relo/Animations/relo-npc_Anim_skeletonreuleaux_telekinesis_taking_right_Montage.relo-npc_Anim_skeletonreuleaux_telekinesis_taking_right_Montage" :!type "AnimMontage Object Reference"))))

(fn `Notify_Attack`
  (returns (Success :type Boolean))
  (locals (DamagedActors :type "Array of Actor Object Reference"))
  (bind _mesh (`self.Mesh`))
  (bind _returnvalue (`SceneComponent.GetSocketLocation` _mesh "SCK_Hand_R"))
  (bind _success (`parent.Notify_Attack`))
  (if _success
    (bind _outhits (`KismetSystemLibrary.SphereTraceMulti` :`Start` _returnvalue :`End` (+ _returnvalue (* (`SceneComponent.GetRightVector` _mesh) 1.0)) :`Radius` 15.0 :`TraceChannel` "TraceTypeQuery2" :`bTraceComplex` true :`DrawTime` 1.0))
    (for _array_element _outhits
      (bind (_bblockinghit _binitialoverlap _time _distance _location _impactpoint _normal _impactnormal _physmat _hitactor) (`GameplayStatics.BreakHitResult` _array_element))
      (if (not (`KismetArrayLibrary.Array_Contains` (`local.DamagedActors`) _hitactor))
        (bind _aspawn (cast `Pawn` _hitactor))
        (if (`self.IsPlayerControlled` _aspawn)
          (`GameplayStatics.ApplyPointDamage` _hitactor (`.Main_Attack_Damage_14_FEA9B05746B12381244B538F3848CF53` (break `/Game/Hell/Core/DATA/Structures/S_AI_Settings` (`self.GetAISettings`))) _normal _array_element (`self.GetController`) self)
          (if (`KismetSystemLibrary.DoesImplementInterface` _hitactor "/Game/Hell/Core/Interfaces/BPI_SkillEffects.BPI_SkillEffects_C")
            (message `/Game/Hell/Core/Interfaces/BPI_SkillEffects.Push` _hitactor (`KismetMathLibrary.Normal` (- (`self.K2_GetActorLocation` _hitactor) (`self.K2_GetActorLocation`))))
            (`self.IncreaseDecreaseWill` true (`.Main_Skill_WillFeedback_16_894274644053CF139CC1D19C110866B8` (break `/Game/Hell/Core/DATA/Structures/S_AI_Settings` (`self.GetAISettings`))))
            (`KismetArrayLibrary.Array_Add` (`local.DamagedActors`) _hitactor)))))
    (return true)
    (else
      (return false))))

(fn `RagdollEffect`
  (params (`On/Off` :type Boolean))
  (returns (Return :type Boolean))
  (`self.RagdollIn` `On/Off`)
  (return `On/Off`))

(fn `ResetAllStates`
  (bind _returnvalue (`SkeletalMeshComponent.GetAnimInstance` (`self.Mesh`)))
  (`parent.ResetAllStates`)
  (`MovementComponent.StopMovementImmediately` (`self.CharacterMovement`))
  (`AnimInstance.Montage_Stop` _returnvalue 0.1 (`AnimInstance.GetCurrentActiveMontage` _returnvalue)))

(fn `Set_GeneralState`
  (params (AI_General_State :type "/Game/Hell/Core/DATA/ENUMS/E_BotStates Enum" :default "NewEnumerator0"))
  (returns (Success :type Boolean))
  (bind _success (`parent.Set_GeneralState` AI_General_State))
  (return _success))

(fn `UserConstructionScript`
  (`parent.UserConstructionScript`))